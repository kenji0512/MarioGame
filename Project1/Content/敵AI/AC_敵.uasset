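; AC_敵 is an enemy AI controller that runs the Bt_敵 behavior tree and feeds it the player as an attack target.
; On BeginPlay it starts the tree and caches the player character as BP_ThirdPersonCharacter.
; When its PawnSensing component sees that pawn, it writes it to the AttackTarget blackboard key; nothing here clears the key.
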(event OnSeePawn(PawnSensing)
  (params (Pawn :type Pawn%20Object%20Reference))
  (bind _player (Variables|Default|Getplayer))
  (if (== Pawn _player)
    (AI|Components|Blackboard|SetValueasObject (Variables|Default|GetBlackboard) (Variables|Default|GetAttack%20Target) _player)))

(event EventBeginPlay
  (AI|RunBehaviorTree "/Game/敵AI/bt_敵.bt_敵")
  (bind _asbp_third_person_character (Utilities|Casting|CastToBP_ThirdPersonCharacter (Game|GetPlayerCharacter 0)))
  (Variables|Default|Setplayer _asbp_third_person_character))

(fn ConstructionScript)